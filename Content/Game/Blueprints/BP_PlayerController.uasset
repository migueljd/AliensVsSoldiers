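; Player controller for tap-to-move control of the BasePlayer character, with automatic facing and attacking of enemies in range.
; A touch trace either sets a tapped BaseEnemy as the character's target or stores the hit point as a movement goal.
; Each tick it moves toward that goal, or follows the target when the goal holds a far-off sentinel value.
; It also faces the next enemy, picking from those in range, and toggles the attack animation.
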(event `InputTouch`
  (params (Location :type "Vector Structure") (FingerIndex :type "ETouchIndex Enum"))
  (bind (_bblockinghit _binitialoverlap _time _location _impactpoint _normal _impactnormal _physmat _hitactor) (`GameplayStatics.BreakHitResult` (`self.GetHitResultUnderCursorForObjects` (`|MakeArray` "ObjectTypeQuery1" "ObjectTypeQuery2" :!type "EObjectTypeQuery Enum") false)))
  ;[1 1 1] Touch Input Logic
  (:`Pressed`
    ;;[1 1 1] If an enemy was hit, the player should move accordingly
    (bind _asbase_enemy (cast `/Game/Game/Blueprints/BaseEnemy` _hitactor)
      (:`then`
        (`KismetSystemLibrary.PrintString` "Setting target")
        (set `/Game/Game/Blueprints/BP_BaseCharacter.Target` _asbase_enemy (`self.PlayerCharacter`))
        (set `self.Goal` (`self.ZeroGoal`)))
      (:`CastFailed`
        ;;[1 1 1] If an enemy wasnt hit, just move to the location
        (set `self.Goal` _impactpoint)))))

(event `self.ReceiveBeginPlay`
  (bind _asbase_player (cast `/Game/Game/Blueprints/BasePlayer` (`GameplayStatics.GetPlayerCharacter` 0)))
  (set `self.PlayerCharacter` _asbase_player)
  (bind _output_get (set `self.ZeroGoal` (-999999.0 -999999.0 -99999.0)))
  (set `self.Goal` _output_get))

(event `self.ReceiveTick`
  (params (DeltaSeconds :type "Float (single-precision)"))
  (bind _playercharacter (`self.PlayerCharacter`))
  (bind _playercharacter_2 (`self.PlayerCharacter`))
  (bind _playercharacter_3 (`self.PlayerCharacter`))
  (bind _target (`/Game/Game/Blueprints/BP_BaseCharacter.Target` (`self.PlayerCharacter`)))
  (`|ExecutionSequence`
    (:`then_0`
      (if (== (`self.Goal`) (`self.ZeroGoal`) :`ErrorTolerance` 0.01)
        (`/Engine/EditorBlueprintResources/StandardMacros.IsValid` _target
          (:`Is Valid`
            (if (>= (`KismetMathLibrary.VSize` (- (`self.K2_GetActorLocation` (`self.PlayerCharacter`)) (`self.K2_GetActorLocation` _target))) 100.0)
              (`NavigationSystem.SimpleMoveToActor` self _target))))
        (elif (not (== (`self.K2_GetActorLocation` (`self.PlayerCharacter`)) (`self.Goal`)))
          (`NavigationSystem.SimpleMoveToLocation` self (`self.Goal`)))))
    (:`then_1`
      (`/Engine/EditorBlueprintResources/StandardMacros.IsValid` (`/Game/Game/Blueprints/BasePlayer.NextEnemyToAttack` _playercharacter_2)
        (:`Is Valid`
          (`/Game/Game/Blueprints/BP_BaseCharacter.LookAt` _playercharacter_3 (`/Game/Game/Blueprints/BasePlayer.NextEnemyToAttack` _playercharacter_3) :!label _label))
        (:`Is Not Valid`
          (if (> (`KismetArrayLibrary.Array_Length` (`/Game/Game/Blueprints/BasePlayer.EnemiesInRange` _playercharacter_2)) 0)
            (set `/Game/Game/Blueprints/BasePlayer.NextEnemyToAttack` (`KismetArrayLibrary.Array_Get` (`/Game/Game/Blueprints/BasePlayer.EnemiesInRange` _playercharacter)) _playercharacter)
            (`/Game/Game/Blueprints/BasePlayer.EnableAttackAnimation` _playercharacter true)
            (goto _label)
            (else
              (`/Game/Game/Blueprints/BasePlayer.EnableAttackAnimation` (`self.PlayerCharacter`) false))))))))

(fn `GetMoveToCursor`
  (returns (IsMovingToCursor :type Boolean))
  (return (`self.bMoveToMouseCursor`)))

(fn `UserConstructionScript`)