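; BasePlayer is the base player character Blueprint, handling enemy targeting and melee-style attacks against BaseEnemy actors.
; Range events maintain EnemiesInRange, promote the chosen Target to NextEnemyToAttack when it enters range, and clear it when it leaves.
; Entry of the Target switches on the attack flag in MixamoAnimBP_Maw; nothing here switches it off.
; Attack applies Damage to NextEnemyToAttack through DealDamage.
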(event `self.ReceiveTick`
  (params (DeltaSeconds :type "Float (single-precision)")))

(event `self.CharacterGotInRange`
  (params (Character :type "/Game/Game/Blueprints/BP_BaseCharacter Object Reference"))
  (bind _target (`self.Target`))
  (bind _asbase_enemy (cast `/Game/Game/Blueprints/BaseEnemy` Character))
  (`KismetArrayLibrary.Array_Add` (`self.EnemiesInRange`) _asbase_enemy)
  (bind _asbase_enemy_2 (cast `/Game/Game/Blueprints/BaseEnemy` _target))
  (if (== _asbase_enemy _target)
    (set `self.NextEnemyToAttack` _asbase_enemy_2)
    (`self.EnableAttackAnimation` true)))

(event `self.CharacterLeftRange`
  (params (Character :type "/Game/Game/Blueprints/BP_BaseCharacter Object Reference"))
  (bind _asbase_enemy (cast `/Game/Game/Blueprints/BaseEnemy` Character))
  (if (== _asbase_enemy (`self.NextEnemyToAttack`))
    (set `self.NextEnemyToAttack` null))
  (`KismetArrayLibrary.Array_RemoveItem` (`self.EnemiesInRange`) _asbase_enemy)
  (if (== (`KismetArrayLibrary.Array_Length` (`self.EnemiesInRange`)) 0)
    _))

(fn `Attack`
  (`self.DealDamage` (`self.NextEnemyToAttack`)))

(fn `DealDamage`
  (params (Enemy :type "/Game/Game/Blueprints/BP_BaseCharacter Object Reference"))
  (`self.TakeDamage` Enemy (`self.Damage`)))

(fn `EnableAttackAnimation`
  (params (AttackEnabled :type Boolean))
  (bind _asmixamo_anim_bp_maw (cast `/Game/MixamoAnimPack/Mixamo_Maw/Anims/MixamoAnimBP_Maw` (`SkeletalMeshComponent.GetAnimInstance` (`self.Mesh`)))
    (:`then`
      (bind _output_get (set `/Game/MixamoAnimPack/Mixamo_Maw/Anims/MixamoAnimBP_Maw.EnableAttack` AttackEnabled _asmixamo_anim_bp_maw))
      (if _output_get
        _))
    (:`CastFailed`
      (`KismetSystemLibrary.PrintString` "The Character animation set is wrong"))))

(fn `SetNewTarget`
  (params (`New Target` :type "/Game/Game/Blueprints/BP_BaseCharacter Object Reference"))
  (set `self.Target` `New Target`))

(fn `UserConstructionScript`
  (`parent.UserConstructionScript`))